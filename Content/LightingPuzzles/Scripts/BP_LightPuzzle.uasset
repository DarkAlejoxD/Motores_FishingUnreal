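; BP_LightPuzzle is a light puzzle actor whose spotlight color the player can cycle while standing nearby.
; On BeginPlay it applies the first LightColor entry and binds to the OnChangeColor dispatcher on the player's BP_ThirdPersonCharacter.
; Sphere overlaps with that character class set PlayerInRadius, which gates the dispatcher response.
; ChangeLightColor advances LightIndex through the color array, wrapping to the start, and updates the SpotLight.
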(event `self.ReceiveBeginPlay`
  (`LightComponent.SetLightColor` (`self.SpotLight`) (`|GetArrayItem` (`self.LightColor`)) true)
  (bind _asbp_third_person_character (cast `/Game/ThirdPerson/Blueprints/BP_ThirdPersonCharacter` (`GameplayStatics.GetPlayerPawn` 0)))
  (add `/Game/ThirdPerson/Blueprints/BP_ThirdPersonCharacter.OnChangeColor` _asbp_third_person_character (delegate `OnChangeColor_Event`)))

(event `OnChangeColor_Event`
  (if (`self.PlayerInRadius`)
    (`self.Change Light Color`)))

(event `self.Sphere.OnComponentBeginOverlap`
  (params (OverlappedComponent :type "PrimitiveComponent Object Reference") (OtherActor :type "Actor Object Reference") (OtherComp :type "PrimitiveComponent Object Reference") (OtherBodyIndex :type Integer) (bFromSweep :type Boolean) (SweepResult :type "HitResult Structure (by ref)"))
  (cast `/Game/ThirdPerson/Blueprints/BP_ThirdPersonCharacter` OtherActor)
  (set `self.PlayerInRadius` true))

(event `self.Sphere.OnComponentEndOverlap`
  (params (OverlappedComponent :type "PrimitiveComponent Object Reference") (OtherActor :type "Actor Object Reference") (OtherComp :type "PrimitiveComponent Object Reference") (OtherBodyIndex :type Integer))
  (cast `/Game/ThirdPerson/Blueprints/BP_ThirdPersonCharacter` OtherActor)
  (set `self.PlayerInRadius` false))

(fn `Change Light Color`
  (bind _result (`/Engine/EditorBlueprintResources/StandardMacros.IncrementInt` (`self.LightIndex`))
    (:`  `
      (if (not (< _result (`KismetArrayLibrary.Array_Length` (`self.LightColor`))))
        (set `self.LightIndex` 0))
      (`LightComponent.SetLightColor` (`self.SpotLight`) (`|GetArrayItem` (`self.LightColor`) (`self.LightIndex`)) true))))

(fn `UserConstructionScript`)