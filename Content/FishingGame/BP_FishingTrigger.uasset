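; Trigger actor for a fishing spot that shows a HUD prompt when the player is inside its sphere and facing its center.
; Each tick, a dot product between the capsule's forward vector and the direction to the center, compared against a minimum threshold, toggles the prompt widget.
; The start-fishing input works only while the prompt shows, calling the character's fishing toggle and widget events.
; While fishing, it hides the prompt and polls the character to detect when fishing ends.
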(event `self.ReceiveBeginPlay`
  (set `self.isFishing` false))

(event `self.ReceiveTick`
  (params (DeltaSeconds :type "Float (single-precision)"))
  ;[1 1 1 0.382] Update
  (if (`self.isFishing`)
    (`self.ToogleFishText` false)
    (bind _asbp_third_person_character (cast `/Game/ThirdPerson/Blueprints/BP_ThirdPersonCharacter` (`GameplayStatics.GetPlayerCharacter` 0)))
    (bind _isfishing (`/Game/ThirdPerson/Blueprints/BP_ThirdPersonCharacter.IsFishing` _asbp_third_person_character))
    (if (not _isfishing)
      (set `self.isFishing` _isfishing))
    (else
      (`self.OnHUDTextUpdate` DeltaSeconds))))

(event `self.Sphere.OnComponentBeginOverlap`
  (params (OverlappedComponent :type "PrimitiveComponent Object Reference") (OtherActor :type "Actor Object Reference") (OtherComp :type "PrimitiveComponent Object Reference") (OtherBodyIndex :type Integer) (bFromSweep :type Boolean) (SweepResult :type "HitResult Structure (by ref)"))
  ;[1 1 1 0.183] Overlap Logic
  (bind _asbp_third_person_character (cast `/Game/ThirdPerson/Blueprints/BP_ThirdPersonCharacter` OtherActor)
    (:`then`
      (set `self.playerInstance` _asbp_third_person_character)
      (set `self.playerNear` true))
    (:`CastFailed`
      (`KismetSystemLibrary.PrintString` "Cast failed"))))

(event `self.Sphere.OnComponentEndOverlap`
  (params (OverlappedComponent :type "PrimitiveComponent Object Reference") (OtherActor :type "Actor Object Reference") (OtherComp :type "PrimitiveComponent Object Reference") (OtherBodyIndex :type Integer))
  ;[1 1 1 0.183] Overlap Logic
  (cast `/Game/ThirdPerson/Blueprints/BP_ThirdPersonCharacter` OtherActor)
  (set `self.playerNear` false))

(event `EnhancedInput|/Game/ThirdPerson/Input/Actions/IA_StartFishing`
  (params (ActionValue :type Boolean) (ElapsedSeconds :type "Float (double-precision)") (TriggeredSeconds :type "Float (double-precision)") (InputAction :type "InputAction Object Reference" :default "/Game/ThirdPerson/Input/Actions/IA_StartFishing.IA_StartFishing"))
  (:`Triggered`
    (if (`self.isFishing`)
      _
      (elif (`self.isDisplayingText`)
        (`/Game/ThirdPerson/Blueprints/BP_ThirdPersonCharacter.ToogleFishingEvent_Event` (`self.playerInstance`) true)
        (set `self.isFishing` true)
        (`/Game/ThirdPerson/Blueprints/BP_ThirdPersonCharacter.OnCreateWidget_Event` (`self.playerInstance`))))))

(fn `OnHUDTextUpdate`
  (params (dt :type "Float (double-precision)"))
  (if (`self.playerNear`)
    (if (>= (`KismetMathLibrary.Dot_VectorVector` (`SceneComponent.GetForwardVector` (`Character.CapsuleComponent` (`self.playerInstance`))) (`KismetMathLibrary.GetDirectionUnitVector` (`SceneComponent.K2_GetComponentLocation` (`Character.CapsuleComponent` (`self.playerInstance`))) (`SceneComponent.K2_GetComponentLocation` (`self.Center`)))) (`self.minDotToFish`))
      (`self.ToogleFishText` true)
      (else
        (`self.ToogleFishText` false :!label _label)))
    (else
      (goto _label))))

(fn `SetTextFalse`
  (if (`self.isDisplayingText`)
    (set `self.isDisplayingText` false)
    (`Widget.RemoveFromParent` (`self.textHUDInstance`))))

(fn `SetTextTrue`
  (if (not (`self.isDisplayingText`))
    (set `self.isDisplayingText` true)
    (bind _returnvalue (`|CreateWidget` "/Game/FishingGame/BP_HUDText.BP_HUDText_C"))
    (`UserWidget.AddToViewport` _returnvalue 0)
    (set `self.textHUDInstance` _returnvalue)))

(fn `ToogleFishText`
  (params (activeValue :type Boolean))
  (if activeValue
    (`self.SetTextTrue`)
    (else
      (`self.SetTextFalse`))))

(fn `UserConstructionScript`)